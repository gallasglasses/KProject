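; BP_WindmillSampo is an interactable windmill actor that spins up a wheel mesh, bursts into particles and removes itself.
; Interact fires the OnStart dispatcher, bound at BeginPlay to Rotate, and reports the interaction finished.
; Chained timers move from rotation to the particle burst, then to destruction.
; Tick rolls the wheel and, after the burst, multiplies the root's scale and Z location by ScaleMesh each frame.
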(event `self.ReceiveBeginPlay`
  (add `self.OnStart` (delegate `Rotate`)))

(event `Rotate`
  (set `self.CanStartRotate` true)
  (bind _returnvalue (`KismetSystemLibrary.K2_SetTimerDelegate` (delegate `Explosion`) 2.0))
  (set `self.Timer` _returnvalue)
  (`KismetSystemLibrary.PrintString` "rotate"))

(event `Explosion`
  (`KismetSystemLibrary.K2_ClearAndInvalidateTimerHandle` (`self.Timer`))
  (`GameplayStatics.SpawnEmitterAttached` (`self.Particle`) (`self.DefaultSceneRoot`) "None" (`self.ParticleLocation`))
  (set `self.CanDestroy` true)
  (bind _returnvalue (`KismetSystemLibrary.K2_SetTimerDelegate` (delegate `Destroy`) 2.0))
  (set `self.Timer` _returnvalue))

(event `Destroy`
  (`KismetSystemLibrary.K2_ClearAndInvalidateTimerHandle` (`self.Timer`))
  (`self.K2_DestroyActor`))

(event `self.ReceiveTick`
  (params (DeltaSeconds :type "Float (single-precision)"))
  (bind _scalemesh (`self.ScaleMesh`))
  (if (`self.CanStartRotate`)
    (`SceneComponent.K2_AddRelativeRotation` (`self.SpinningMesh`) (`KismetMathLibrary.MakeRotator` (`self.RotationSpeedWheel`)) false false)
    (if (`self.CanDestroy`)
      (`SceneComponent.K2_SetWorldTransform` (`self.DefaultSceneRoot`) (`KismetMathLibrary.MakeTransform` (`KismetMathLibrary.MakeVector` (.x (.location (`SceneComponent.K2_GetComponentToWorld` (`self.DefaultSceneRoot`)))) (.y (.location (`SceneComponent.K2_GetComponentToWorld` (`self.DefaultSceneRoot`)))) (* (.z (.location (`SceneComponent.K2_GetComponentToWorld` (`self.DefaultSceneRoot`)))) _scalemesh)) (.rotation (`SceneComponent.K2_GetComponentToWorld` (`self.DefaultSceneRoot`))) (* (.scale (`SceneComponent.K2_GetComponentToWorld` (`self.DefaultSceneRoot`))) _scalemesh)) false false))))

(event `self.Interact`
  (params (ActorInteractedWithObject :type "Actor Object Reference"))
  (`self.OnStart`)
  (`self.OnInteractionFinished` ActorInteractedWithObject))

(fn `UserConstructionScript`)